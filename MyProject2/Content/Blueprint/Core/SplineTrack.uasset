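; Spline track actor that carries the first-person player along its path, hanging below the spline like a zipline.
; Construction script builds spline mesh segments between points and positions the StartPoint and EndPoint markers.
; Overlapping StartPoint enables input, so Interact starts a timeline at a configurable play rate.
; The timeline curve maps to spline distance, teleporting the player each update, lowered by capsule half-height and a ride offset.
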(event `self.ReceiveBeginPlay`
  ;[1 1 1] Event Begin Play
  (bind _asfirst_person_character (cast `/Game/FirstPersonBP/Blueprints/FirstPersonCharacter` (`GameplayStatics.GetPlayerCharacter` 0)))
  (set `self.PlayerRef` _asfirst_person_character)
  (`TimelineComponent.SetPlayRate` (`self.Timeline`) (`self.PlayRate`)))

(event `InputAction|Interact`
  (params (Key :type "Key Structure" :default "AnyKey"))
  ;[1 1 1] Track Movement
  (:`Pressed`
    (`/Engine/EditorBlueprintResources/StandardMacros.DoOnce` false :!label _label
      (:`Completed`
        (bind (_direction _spline_curve) (`Timeline|Timeline` :`NewTime` 0.2 :!via `PlayFromStart`)
          (:`Update`
            (`self.SplineReset`)
            (`self.K2_SetActorLocation` (`self.PlayerRef`) (`KismetMathLibrary.MakeVector` (.x (`SplineComponent.GetLocationAtDistanceAlongSpline` (`self.Spline`) (* _spline_curve (`SplineComponent.GetSplineLength` (`self.Spline`))) "World")) (.y (`SplineComponent.GetLocationAtDistanceAlongSpline` (`self.Spline`) (* _spline_curve (`SplineComponent.GetSplineLength` (`self.Spline`))) "World")) (- (- (.z (`SplineComponent.GetLocationAtDistanceAlongSpline` (`self.Spline`) (* _spline_curve (`SplineComponent.GetSplineLength` (`self.Spline`))) "World")) (`CapsuleComponent.GetScaledCapsuleHalfHeight` (`Character.CapsuleComponent` (`self.PlayerRef`)))) (`self.PlayerSplineRideOffset`))) false true)))))))

(event `SplineReset`
  ;[1 1 1] Track Movement
  (goto _label :!via `Reset`))

(event `self.StartPoint.OnComponentBeginOverlap`
  (params (OverlappedComponent :type "PrimitiveComponent Object Reference") (OtherActor :type "Actor Object Reference") (OtherComp :type "PrimitiveComponent Object Reference") (OtherBodyIndex :type Integer) (bFromSweep :type Boolean) (SweepResult :type "HitResult Structure (by ref)"))
  ;[1 1 1] Track Trigger
  (cast `/Game/FirstPersonBP/Blueprints/FirstPersonCharacter` OtherActor)
  (`self.EnableInput` (`GameplayStatics.GetPlayerController` 0)))

(event `self.StartPoint.OnComponentEndOverlap`
  (params (OverlappedComponent :type "PrimitiveComponent Object Reference") (OtherActor :type "Actor Object Reference") (OtherComp :type "PrimitiveComponent Object Reference") (OtherBodyIndex :type Integer))
  ;[1 1 1] Track Trigger
  (cast `/Game/FirstPersonBP/Blueprints/FirstPersonCharacter` OtherActor)
  (`self.DisableInput` (`GameplayStatics.GetPlayerController` 0)))

(fn `UserConstructionScript`
  (bind _returnvalue (`SplineComponent.GetNumberOfSplinePoints` (`self.Spline`)))
  (for _index (range (+ (- _returnvalue 2) 1))
    (`SceneComponent.K2_SetRelativeLocation` (`self.StartPoint`) (`SplineComponent.GetLocationAndTangentAtSplinePoint` (`self.Spline`) (`|GetArrayItem` (`|MakeArray` _returnvalue) _returnvalue) "Local") false false)
    (`SceneComponent.K2_SetRelativeLocation` (`self.EndPoint`) (`SplineComponent.GetLocationAndTangentAtSplinePoint` (`self.Spline`) (`|GetArrayItem` (`|MakeArray` _returnvalue)) "Local") false false)
    (bind _returnvalue_2 (`AddComponent|NODE_AddSplineMeshComponent-0`))
    (`SceneComponent.K2_AttachToComponent` (`self.DefaultSceneRoot`) _returnvalue_2 "None" "KeepRelative" "KeepRelative" "KeepRelative" true)
    (bind (_location _tangent) (`SplineComponent.GetLocationAndTangentAtSplinePoint` (`self.Spline`) _index "Local"))
    (bind (_location_2 _tangent_2) (`SplineComponent.GetLocationAndTangentAtSplinePoint` (`self.Spline`) (+ _index 1) "Local"))
    (`SplineMeshComponent.SetStartAndEnd` _returnvalue_2 _location _tangent _location_2 _tangent_2 true)))