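; Base enemy Blueprint that attacks the player and is destroyed when a FirstPersonProjectile overlaps it.
; StartAttacking runs Attack on a looping one-second timer, which StopAttacking clears.
; Each Attack line-traces on Visibility to the player, with debug drawing left on, and subtracts Damage directly from the character's CurrHealth if the trace hits a FirstPersonCharacter.
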(event `self.ReceiveActorBeginOverlap`
  (params (OtherActor :type "Actor Object Reference"))
  (cast `/Game/FirstPersonBP/Blueprints/FirstPersonProjectile` OtherActor)
  (if true
    (`self.K2_DestroyActor`)))

(event `StartAttacking`
  (`KismetSystemLibrary.K2_SetTimer` null "Attack" 1.0 true))

(event `Attack`
  (bind (_outhit _returnvalue) (`KismetSystemLibrary.LineTraceSingle` :`Start` (`self.K2_GetActorLocation`) :`End` (`self.K2_GetActorLocation` (`GameplayStatics.GetPlayerCharacter` 0)) :`TraceChannel` "TraceTypeQuery1" :`DrawDebugType` "ForDuration"))
  (if _returnvalue
    (bind _asfirst_person_character (cast `/Game/FirstPersonBP/Blueprints/FirstPersonCharacter` (`.HitActor` (`GameplayStatics.BreakHitResult` _outhit))))
    (set `/Game/FirstPersonBP/Blueprints/FirstPersonCharacter.CurrHealth` (- (`/Game/FirstPersonBP/Blueprints/FirstPersonCharacter.CurrHealth` _asfirst_person_character) (`self.Damage`)) _asfirst_person_character)))

(event `StopAttacking`
  (`KismetSystemLibrary.K2_ClearTimer` null "Attack"))

(fn `UserConstructionScript`)