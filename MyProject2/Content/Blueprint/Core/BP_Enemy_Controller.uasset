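; AI controller for enemies derived from BP_Enemy_Base, which runs the AI_BT behavior tree when possessing one.
; Perception updates on the FirstPersonCharacter write the sensed result to the CanSeePlayer blackboard key.
; The same result tells the controlled enemy to start attacking when the player is sensed and to stop when sensing is lost.
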(event `self.OnPossess`
  (params (PossessedPawn :type "Pawn Object Reference"))
  (cast `/Game/Blueprint/Core/BP_Enemy_Base` PossessedPawn)
  (`self.RunBehaviorTree` "/Game/Blueprint/Core/AI/AI_BT.AI_BT"))

(event `self.AIPerception.OnTargetPerceptionUpdated`
  (params (Actor :type "Actor Object Reference") (Stimulus :type "AIStimulus Structure"))
  (bind (_age _expirationage _strength _stimuluslocation _receiverlocation _tag _bsuccessfullysensed) (break `AIStimulus` Stimulus))
  (bind _returnvalue (`self.K2_GetPawn`))
  (cast `/Game/FirstPersonBP/Blueprints/FirstPersonCharacter` Actor)
  (`BlackboardComponent.SetValueAsBool` (`AIBlueprintHelperLibrary.GetBlackboard` null) "CanSeePlayer" _bsuccessfullysensed)
  (if _bsuccessfullysensed
    (bind _asbp_enemy_base (cast `/Game/Blueprint/Core/BP_Enemy_Base` _returnvalue))
    (`/Game/Blueprint/Core/BP_Enemy_Base.StartAttacking` _asbp_enemy_base)
    (else
      (bind _asbp_enemy_base_2 (cast `/Game/Blueprint/Core/BP_Enemy_Base` _returnvalue))
      (`/Game/Blueprint/Core/BP_Enemy_Base.StopAttacking` _asbp_enemy_base_2))))

(fn `UserConstructionScript`)